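; A sliceable beat target that splits in two when hit, extending its parent's overlap handling.
; The construction script copies the static BeatMesh into a procedural mesh with collision.
; On first overlap, it slices that mesh along the hit direction, capping the cut with the hit-side mesh's material.
; Both halves get physics and opposing randomized impulses, then the actor destroys itself after a short delay.
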(event EventOnBeatOverlap
  (params (HitDirection :type Vector :default "0, 0, 0") (Impulse :type Vector :default "0, 0, 0"))
  (bind _returnvalue (Math|Random|RandomFloatinRange 0.0 3e+02))
  (bind _returnvalue_2 (Math|Random|RandomFloatinRange 0.0 3e+02))
  (bind _hitsidemesh (Variables|Default|GetHitSideMesh))
  ;[1 1 1] Slicing Beat
  (|CallParentFunction HitDirection Impulse)
  (Utilities|FlowControl|DoOnce false
    (:Completed
      (Physics|SetSimulatePhysics (Variables|Default|GetProcedualMesh) true)
      (Physics|AddImpulse (Variables|Default|GetProcedualMesh) (+ (* Impulse -1.0) (Math|Vector|MakeVector _returnvalue_2 _returnvalue_2 _returnvalue_2)) "None" true)
      (Utilities|IsValid _hitsidemesh
        (:Is%20Valid
          (bind _outotherhalfprocmesh (Class|KismetProceduralMeshLibrary|SliceProceduralMesh (Variables|Default|GetProcedualMesh) (Transformation|GetWorldLocation (Variables|Default|GetProcedualMesh)) HitDirection true "CreateNewSectionForCap" (Rendering|Material|GetMaterial _hitsidemesh 0)))
          (Physics|SetSimulatePhysics _outotherhalfprocmesh true)
          (Physics|AddImpulse _outotherhalfprocmesh (+ Impulse (Math|Vector|MakeVector _returnvalue _returnvalue _returnvalue)) "None" true)
          (Utilities|IsValid (Variables|Default|GetHitSideMesh)
            (:Is%20Valid
              (Components|DestroyComponent (Variables|Default|GetHitSideMesh))
              (Utilities|FlowControl|Delay 1.0))))
        (:Is%20Not%20Valid
          _))
      (Actor|DestroyActor))))

(fn ConstructionScript
  (Class|KismetProceduralMeshLibrary|CopyProceduralMeshfromStaticMeshComponent (Variables|Default|GetBeatMesh) 0 (Variables|Default|GetProcedualMesh) true))